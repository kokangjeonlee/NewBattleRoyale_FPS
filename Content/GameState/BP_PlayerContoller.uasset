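; Player controller that manages the HUD and world map and applies out-of-zone damage to the controlled pawn.
; It creates the HUD on BeginPlay, and the Worldmap input flip-flops between that and a lazily created, cached map widget.
; About once a second, Tick compares the pawn's horizontal distance to the game state's current scaled circle radius and damages it outside.
; GetPawnPosition returns the pawn location and map size, with a far-off fallback when no pawn exists.
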(event EventTick
  (params (DeltaSeconds :type Float%20%28single-precision%29))
  (bind _returnvalue (Pawn|GetControlledPawn))
  (bind _returnvalue_2 (Transformation|GetActorLocation _returnvalue))
  (bind (_x _y) (Math|Vector|BreakVector _returnvalue_2))
  (bind _output_get (Variables|Default|SetElectricDamagingTime (+ DeltaSeconds (Variables|Default|GetElectricDamagingTime))))
  (if (> _output_get 1.0)
    (Variables|Default|SetElectricDamagingTime 0.0)
    (bind _asbp_game_state_base (Utilities|Casting|CastToBP_GameStateBase (Game|GetGameState)))
    (if (>= (Math|Vector|VectorLength (- (Math|Vector|MakeVector _x _y 0.0) (Math|Vector|MakeVector (.X (Math|Vector|BreakVector (Variables|/Game/GameState/BP_GameStateBase.BP_GameStateBase_C|GetCurrentCirclePosition _asbp_game_state_base))) (.Y (Math|Vector|BreakVector (Variables|/Game/GameState/BP_GameStateBase.BP_GameStateBase_C|GetCurrentCirclePosition _asbp_game_state_base))) 0.0))) (* (Variables|/Game/GameState/BP_GameStateBase.BP_GameStateBase_C|GetCurrentCircleRadius _asbp_game_state_base) 1e+01))
      (bind _asbp_nbrbase_pawn (Utilities|Casting|CastToBP_NBRBasePawn _returnvalue))
      (Default|Damaged _asbp_nbrbase_pawn 2e+01))))

(event EventBeginPlay
  (bind _self self)
  (bind _returnvalue (UserInterface|CreateWidget "/Game/UI/InGameHUD/HUD.HUD_C" _self _self))
  (UserInterface|Viewport|AddtoViewport _returnvalue 0)
  (Variables|Default|SetWidgetBP_HUD _returnvalue))

(event Input|ActionEvents|InputActionWorldmap
  (params (Key :type Key%20Structure))
  (bind _self self)
  (:Pressed
    (Utilities|FlowControl|FlipFlop
      (:A
        (Utilities|IsValid (Variables|Default|GetWidgetBP_Worldmap)
          (:Is%20Valid
            (UserInterface|Viewport|AddtoViewport (Variables|Default|GetWidgetBP_Worldmap) 0)
            (Widget|RemovefromParent (Variables|Default|GetWidgetBP_HUD)))
          (:Is%20Not%20Valid
            (bind _returnvalue (UserInterface|CreateWidget "/Game/Worldmap/WidgetBP_Worldmap.WidgetBP_Worldmap_C" _self _self))
            (bind _output_get (Variables|Default|SetWidgetBP_Worldmap _returnvalue))
            (UserInterface|Viewport|AddtoViewport _output_get 0)
            (Widget|RemovefromParent (Variables|Default|GetWidgetBP_HUD)))))
      (:B
        (Utilities|IsValid (Variables|Default|GetWidgetBP_Worldmap)
          (:Is%20Valid
            (Widget|RemovefromParent (Variables|Default|GetWidgetBP_Worldmap))
            (UserInterface|Viewport|AddtoViewport (Variables|Default|GetWidgetBP_HUD) 0)))))))

(fn ConstructionScript)

(fn GetPawnPosition
  (bind _returnvalue (Pawn|GetControlledPawn))
  (Utilities|IsValid _returnvalue
    (:Is%20Valid
      (return (Transformation|GetActorLocation _returnvalue) (Variables|Default|GetMapSize)))
    (:Is%20Not%20Valid
      (return "100000000376832.000000,100000000376832.000000,0.000000" (Variables|Default|GetMapSize)))))