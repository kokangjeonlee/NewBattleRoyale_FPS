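; BP_PlayerState is a player state Blueprint holding an unfinished stub that appears intended for character selection.
; NewFunction_0 chains comparisons against Sian, Murdock, Trapper and Wraith, but only the first reads the Character input and no branch performs an action.
; BeginPlay, Tick and the construction script are empty.
; An unwired PlayerStart cast and debug prints about changing the default pawn and character never run.
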(event EventBeginPlay)

(event EventTick
  (params (DeltaSeconds :type Float%20%28single-precision%29)))

(fn ConstructionScript)

(fn NewFunction0
  (params (character :type String))
  (if (not (Utilities|Enum|Equal(Enum) character (Variables|Default|GetSian)))
    (if (not (Utilities|Enum|Equal(Enum) "" (Variables|Default|GetMurdock)))
      (if (not (Utilities|Enum|Equal(Enum) "" (Variables|Default|GetTrapper)))
        (if (Utilities|Enum|Equal(Enum) "" (Variables|Default|GetWraith))
          _)))))