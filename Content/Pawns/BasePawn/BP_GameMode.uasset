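; BP_GameMode is a game mode Blueprint with a rough, unfinished function for switching the player's character.
; ChangeDefaultPawn destroys player controller 0, then branches on Sian, Murdock, Trapper or Wraith to set Character to that same value and print debug text.
; It neither spawns a pawn nor assigns a default pawn class.
; ChangeDefaultWeapon, BeginPlay, Tick and the construction script are empty.
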(event EventBeginPlay)

(event EventTick
  (params (DeltaSeconds :type Float%20%28single-precision%29)))

(fn ConstructionScript)

(fn ChangeDefaultPawn
  (params (character :type String))
  (bind _sian (LocalVariables|GetSian))
  (bind _trapper (LocalVariables|GetTrapper))
  (bind _murdock (LocalVariables|GetMurdock))
  (bind _wraith (LocalVariables|GetWraith))
  (Development|PrintString "Im in change default pawn")
  (Actor|DestroyActor (Game|GetPlayerController 0))
  (if (Utilities|Enum|Equal(Enum) character _sian)
    (Variables|Default|Setcharacter _sian)
    (Development|PrintString "change characeter" :!label _label)
    (elif (Utilities|Enum|Equal(Enum) character _murdock)
      (Variables|Default|Setcharacter _murdock)
      (goto _label)
      (elif (Utilities|Enum|Equal(Enum) character _trapper)
        (Variables|Default|Setcharacter _trapper)
        (goto _label)
        (elif (Utilities|Enum|Equal(Enum) character _wraith)
          (Variables|Default|Setcharacter _wraith)
          (goto _label))))))

(fn ChangeDefaultWeapon)