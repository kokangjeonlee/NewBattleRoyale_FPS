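; Player controller Blueprint that creates the HUD and toggles a world map widget.
; StartGame adds the HUD to the viewport, while the Worldmap input uses a FlipFlop to show or remove the map.
; The map widget is created on first use with a controller reference, then cached.
; GetPawnPosition returns the controlled pawn's location and MapSize, substituting a huge off-map position when no pawn is valid.
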(event Custom|StartGame
  (bind _returnvalue (UserInterface|CreateWidget "/Game/UI/InGameHUD/HUD.HUD_C" self))
  (UserInterface|Viewport|AddtoViewport _returnvalue 0))

(event Input|ActionEvents|InputActionWorldmap
  (params (Key :type Key%20Structure))
  (bind _self self)
  (:Pressed
    (Utilities|FlowControl|FlipFlop
      (:A
        (Utilities|IsValid (Variables|Default|GetWidgetBP_Worldmap)
          (:Is%20Valid
            (UserInterface|Viewport|AddtoViewport (Variables|Default|GetWidgetBP_Worldmap) 0))
          (:Is%20Not%20Valid
            (bind _returnvalue (UserInterface|CreateWidget "/Game/Worldmap/WidgetBP_Worldmap.WidgetBP_Worldmap_C" _self _self))
            (bind _output_get (Variables|Default|SetWidgetBP_Worldmap _returnvalue))
            (UserInterface|Viewport|AddtoViewport _output_get 0))))
      (:B
        (Utilities|IsValid (Variables|Default|GetWidgetBP_Worldmap)
          (:Is%20Valid
            (Widget|RemovefromParent (Variables|Default|GetWidgetBP_Worldmap))))))))

(fn ConstructionScript)

(fn GetPawnPosition
  (bind _returnvalue (Pawn|GetControlledPawn))
  (Utilities|IsValid _returnvalue
    (:Is%20Valid
      (return (Transformation|GetActorLocation _returnvalue) (Variables|Default|GetMapSize)))
    (:Is%20Not%20Valid
      (return "100000000376832.000000,100000000376832.000000,0.000000" (Variables|Default|GetMapSize)))))