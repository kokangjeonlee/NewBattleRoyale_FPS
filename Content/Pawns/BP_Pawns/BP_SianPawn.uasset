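; BP_SianPawn is a character pawn with two weapons, a dynamic crosshair and regenerating health.
; On BeginPlay it sets walk speed, creates the crosshair widget, and attaches spawned primary and secondary weapons to hand and holster sockets, equipping the primary.
; Tick flags death at zero health and widens the crosshair with velocity.
; A Delay inside Tick throttles small health increments, with no check for death.
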(event EventBeginPlay
  (bind _mesh (Variables|Character|GetMesh))
  (Variables|/Script/Engine.CharacterMovementComponent|SetMaxWalkSpeed (Variables|Character|GetCharacterMovement) 1.5e+02)
  (bind _returnvalue (UserInterface|CreateWidget "/Game/UI/InGameHUD/WBCrosshair.WBCrosshair_C"))
  (Variables|Default|SetCrosshairRef _returnvalue)
  (UserInterface|Viewport|AddtoViewport _returnvalue 0)
  (Utilities|FlowControl|Sequence
    (:then_0
      (bind _returnvalue_2 (Game|SpawnActorfromClass "/Game/Weapon/BP_WeaponBase.BP_WeaponBase_C" (Math|Transform|MakeTransform "0, 0, 0") "Undefined" 0 0))
      (bind _output_get (Variables|Default|SetPrimaryWeapon _returnvalue_2))
      (Variables|/Game/Weapon/BP_WeaponBase.BP_WeaponBase_C|SetWeaponState _output_get "NewEnumerator0")
      (Transformation|AttachComponentToComponent (Variables|Default|GetPrimaryWeapon) _mesh "Weapon" "KeepRelative" "KeepRelative" "KeepRelative" true))
    (:then_1
      (Variables|Default|SetEquipedWeapon (Variables|Default|GetPrimaryWeapon)))
    (:then_2
      (bind _returnvalue_3 (Game|SpawnActorfromClass "/Game/Weapon/BP_SecondaryWeapon.BP_SecondaryWeapon_C" (Math|Transform|MakeTransform "0, 0, 0") "Undefined" 0 0))
      (bind _output_get_2 (Variables|Default|SetSecondaryWeapon _returnvalue_3))
      (Variables|/Game/Weapon/BP_WeaponBase.BP_WeaponBase_C|SetWeaponState _output_get_2 "NewEnumerator1")
      (Transformation|AttachComponentToComponent (Variables|Default|GetSecondaryWeapon) _mesh "SWHolster" "KeepRelative" "KeepRelative" "KeepRelative" true))))

(event EventTick
  (params (DeltaSeconds :type Float%20%28single-precision%29))
  (Utilities|FlowControl|Sequence
    (:then_0
      (if (<= (Variables|Default|GetHealthPoint) 0.0)
        (Variables|Default|SetIsDead true)))
    (:then_1
      (Utilities|FlowControl|Delay 5.0)
      (if (< (Variables|Default|GetHealthPoint) 1.0)
        (Variables|Default|SetHealthPoint (+ (Variables|Default|GetHealthPoint) 0.02))))
    (:then_2
      (Variables|/Game/UI/InGameHUD/WBCrosshair.WBCrosshair_C|Setcrosshair_spread (Variables|Default|GetCrosshairRef) (Math|Float|MapRangeClamped (Math|Vector|VectorLength (Transformation|GetVelocity)) 0.0 4.5e+02 5.0 8e+01)))))

(event Collision|EventActorBeginOverlap
  (params (OtherActor :type Actor%20Object%20Reference)))

(fn ConstructionScript
  (|CallParentFunction))