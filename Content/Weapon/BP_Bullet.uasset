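; BP_Bullet is a weapon projectile actor that flies straight and destroys itself on hitting a pawn.
; Tick offsets it along the Arrow's forward vector at a fixed speed, without sweep.
; Hit calls DestroyActor only when the other actor's class is exactly BP_NBRBasePawn, and applies no damage.
; SettingBullet is an empty event; the damage setup and timed falloff with a minimum clamp are disconnected and never run.
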(event Custom|SettingBullet
  (params (Damage :type Integer) (DamageFall :type Integer))
  ;[1 1 1] SettingInfo
)

(event EventTick
  (params (DeltaSeconds :type Float%20%28single-precision%29))
  ;[1 1 1] Move
  (Transformation|AddActorWorldOffset (* (Math|Conversions|ToVector(Float) (* DeltaSeconds 1e+02)) (Math|Vector|GetForwardVector (Variables|Default|GetArrow)))))

(event Collision|EventHit
  (params (MyComp :type Primitive%20Component%20Object%20Reference) (Other :type Actor%20Object%20Reference) (OtherComp :type Primitive%20Component%20Object%20Reference) (bSelfMoved :type Boolean) (HitLocation :type Vector :default "0, 0, 0") (HitNormal :type Vector :default "0, 0, 0") (NormalImpulse :type Vector :default "0, 0, 0") (Hit :type Hit%20Result%20Structure%20%28by%20ref%29))
  ;[1 1 1] Hit
  (if (== (Utilities|GetClass Other) "/Game/Pawns/BasePawn/BP_NBRBasePawn.BP_NBRBasePawn_C")
    (Actor|DestroyActor)))

(fn ConstructionScript)